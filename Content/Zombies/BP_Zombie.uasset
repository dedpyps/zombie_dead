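; BP_Zombie is a zombie that chases the player and attacks on reaching it.
; From BeginPlay, ChasePlayer sets IsRunning and runs AIMoveTo toward the first player controller actor, rather than its pawn.
; A successful move plays a sped-up attack montage and clears IsRunning.
; Montage completion or a failed move calls ChasePlayer again, forming an endless chase-attack loop without a behavior tree.
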(event Custom|ChasePlayer
  (Variables|Default|SetisRunning true)
  (AI|AIMoveTo self "0, 0, 0" (Game|GetPlayerController 0) 1e+02 false
    (:OnSuccess
      (Animation|Montage|PlayMontage (Variables|Character|GetMesh) "/Game/Zombies/AS_Zombie_Attack_Montage.AS_Zombie_Attack_Montage" 1.5
        (:then
          (Variables|Default|SetisRunning false))
        (:OnCompleted
          (CallFunction|ChasePlayer))))
    (:OnFail
      (CallFunction|ChasePlayer))))

(event EventBeginPlay
  (CallFunction|ChasePlayer))

(fn ConstructionScript)